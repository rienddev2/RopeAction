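; LeftRight_BP is an actor that moves itself along the world X axis, between its placed location and a point offset by a distance variable (이동거리).
; On BeginPlay it stores both endpoints, then waits a short random delay, so instances can start out of step.
; A Timeline then drives a Lerp between the endpoints, setting the actor location on each update without sweep.
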(event EventBeginPlay
  (bind _output_get (Variables|Default|Set시작위치 (Transformation|GetActorLocation)))
  (Variables|Default|Set도착위치 (+ _output_get (Math|Vector|MakeVector (Variables|Default|Get이동거리) 0.0 0.0)))
  (Utilities|FlowControl|Delay (Math|Random|RandomFloatinRange 0.0 3.0))
  (bind _새_트랙_6 (Timeline|타임라인_0 Play)
    (:Update
      (Transformation|SetActorLocation (Math|Vector|Lerp(Vector) (Variables|Default|Get시작위치) (Variables|Default|Get도착위치) _새_트랙_6) false false))))

(event Collision|EventActorBeginOverlap
  (params (OtherActor :type Actor%20Object%20Reference)))

(event EventTick
  (params (DeltaSeconds :type Float%20%28single-precision%29)))

(fn ConstructionScript)